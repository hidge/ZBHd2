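; Test AI actor that appears to prototype crawling over surfaces by snapping itself to trace hits.
; A delayed Tick traces forward, otherwise down, plus backward when a second down probe misses; most traces ignore Landscape.
; ChangeLocation moves it to the impact point facing along the normal, even for unchecked down and back misses.
; Replicated-style AI MoveTo events are unfinished: Move and BeginPlay are empty, and the authority switch never runs.
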(event Custom|Move)

(event Custom|Move_Client
  (bind _self self)
  (bind _returnvalue (AI|GetAIController _self))
  (AI|AIMoveTo _returnvalue (+ (Transformation|GetWorldLocation (Variables|Collision|GetCapsuleComponent _self)) (* (Transformation|GetActorForwardVector _self) 2.5e+02)) 0 -1.0 "Default" "Default" true true
    (:OnRequestFailed
      _)
    (:OnMoveFinished
      _))
  (CallFunction|Move))

(event Custom|Move_Server
  (CallFunction|MoveClient))

(event EventBeginPlay)

(event EventTick
  (params (DeltaSeconds :type Float%20%28single-precision%29))
  (bind _forward (Variables|Default|GetForward))
  (bind _down (Variables|Default|GetDown))
  (bind _back (Variables|Default|GetBack))
  (bind _down_2 (Variables|Default|GetDown_2))
  (bind _returnvalue (Transformation|GetWorldLocation _back))
  (bind _returnvalue_2 (Transformation|GetWorldLocation _down_2))
  (bind _returnvalue_3 (Transformation|GetWorldLocation _forward))
  (bind _returnvalue_4 (Transformation|GetWorldLocation _down))
  (Utilities|FlowControl|Delay 0.05)
  (bind _outactors (Actor|GetAllActorsOfClass "/Script/Landscape.Landscape"))
  (bind (_outhit _returnvalue_5) (Collision|LineTraceByChannel _returnvalue_3 (+ _returnvalue_3 (* (Math|Vector|GetForwardVector _forward) 25.0)) "TraceTypeQuery1" false _outactors "ForDuration"))
  (if _returnvalue_5
    (CallFunction|ChangeLocation _outhit)
    (else
      (bind _outhit_2 (Collision|LineTraceByChannel _returnvalue_4 (+ _returnvalue_4 (* (Math|Vector|GetForwardVector _down) 25.0)) "TraceTypeQuery1" false _outactors "None"))
      (CallFunction|ChangeLocation _outhit_2)
      (bind _returnvalue_6 (Collision|LineTraceByChannel _returnvalue_2 (+ _returnvalue_2 (* (Math|Vector|GetForwardVector _down_2) 25.0)) "TraceTypeQuery1" false 0 "None"))
      (if (not _returnvalue_6)
        (bind _outhit_3 (Collision|LineTraceByChannel _returnvalue (+ _returnvalue (* (Math|Vector|GetForwardVector _back) 15.0)) "TraceTypeQuery1" false _outactors "None"))
        (CallFunction|ChangeLocation _outhit_3)))))

(fn ConstructionScript)

(fn ChangeLocation
  (params (Hit :type Hit%20Result%20Structure))
  (bind (_bblockinghit _binitialoverlap _time _location _impactpoint _normal _impactnormal) (Collision|BreakHitResult Hit))
  (Transformation|SetActorLocationAndRotation _impactpoint (Math|Rotator|MakeRotationfromAxes _impactnormal "0, 0, 0" "0, 0, 0")))